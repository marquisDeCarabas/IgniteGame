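; Game mode that handles player death and respawn at a saved checkpoint transform, initially the player's starting transform.
; It binds to the player character's destroyed event, then counts the death, notifies any active projectile, and spawns and possesses a replacement character.
; Each new character is re-bound, and camera fade-out and fade-in are issued in the same pass with no delay.
; Time and death debug prints are unwired; EndDemo is empty.
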(event `EndDemo`)

(event `self.ReceiveBeginPlay`
  (`self.Respawn`)
  (set `self.transform_checkPoint` (`self.GetTransform` (`GameplayStatics.GetPlayerCharacter` 0)))
  (set `self.i_nDeaths` 0))

(event `Respawn`
  (bind _asplayer_char (cast `/Game/Player/player_char` (`GameplayStatics.GetPlayerCharacter` 0)))
  (bind _output_get (set `self.player` _asplayer_char))
  (add `self.OnDestroyed` _output_get (delegate `Destroyed_`)))

(event `Destroyed_` :!signature `self.OnDestroyed`
  (params (DestroyedActor :type "Actor Object Reference"))
  (`/Engine/EditorBlueprintResources/StandardMacros.IncrementInt` (`self.i_nDeaths`)
    (:`  `
      (bind _a_projectile (`/Game/Player/player_char.a_projectile` (`self.player`))
        (:`then`
          (`/Game/Player/projectile_actor.PlayerDied` _a_projectile))
        (:`else`
          _))
      (`PlayerCameraManager.StartCameraFade` :`self` (`GameplayStatics.GetPlayerCameraManager` 0) :`ToAlpha` 1.0 :`Duration` 0.5)
      (bind _returnvalue (`|SpawnActorFromClass` "/Game/Player/player_char.player_char_C" (`self.transform_checkPoint`) "AdjustIfPossibleButAlwaysSpawn" "OverrideRootScale" null null))
      (`/Engine/EditorBlueprintResources/StandardMacros.IsValid` _returnvalue
        (:`Is Valid`
          (`/Game/Player/player_char.Respawner` _returnvalue)
          (`Controller.Possess` (`GameplayStatics.GetPlayerController` 0) _returnvalue)
          (`self.Respawn`)
          (`PlayerCameraManager.StartCameraFade` :`self` (`GameplayStatics.GetPlayerCameraManager` 0) :`FromAlpha` 1.0 :`Duration` 0.5))))))

(event `self.ReceiveTick`
  (params (DeltaSeconds :type "Float (single-precision)")))

(fn `UserConstructionScript`)